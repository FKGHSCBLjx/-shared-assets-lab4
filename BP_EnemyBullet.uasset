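; BP_EnemyBullet is an enemy projectile that damages the player's tank on contact.
; On begin play it caches the player character as a BP_MainTank reference.
; When its sphere overlaps an actor tagged MainTank it calls that tank's DamageSystem with its Damage value and destroys itself.
; Overlapping any other actor destroys it after a fixed delay instead.
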(event OnComponentBeginOverlap(Sphere)
  (params (OverlappedComponent :type Primitive%20Component%20Object%20Reference) (OtherActor :type Actor%20Object%20Reference) (OtherComp :type Primitive%20Component%20Object%20Reference) (OtherBodyIndex :type Integer) (bFromSweep :type Boolean) (SweepResult :type Hit%20Result%20Structure%20%28by%20ref%29))
  ;[0.4678 0 0.3937] Checking For Tag
  (if (Actor|ActorHasTag OtherActor "MainTank")
    ;[0 1 0.1046] Causing Damage To Player
    (Default|DamageSystem (Variables|Default|GetAs%20BP%20Main%20Tank) (Variables|Default|GetDamage))
    (else
      (Utilities|FlowControl|Delay 15.0)))
  (Actor|DestroyActor))

(event EventBeginPlay
  ;[1 0.896 0] Creating Player Reference
  (bind _asbp_main_tank (Utilities|Casting|CastToBP_MainTank (Game|GetPlayerCharacter 0)))
  (Variables|Default|SetAs%20BP%20Main%20Tank _asbp_main_tank))

(fn ConstructionScript)